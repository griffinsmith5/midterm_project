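; Player pawn that moves via a Sphere component and wins the game on reaching a fixed score set at BeginPlay.
; Four input axes feed AddMovementInput along the sphere's forward and right vectors, negated for opposite directions.
; Tick checks Score against WinScore, then shows the Victory widget, pauses, shows the cursor and increments Lives.
; Pressing Q adds a Pause widget to the viewport without pausing the game itself.
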(event `Key|Q`
  (params (Key :type "Key Structure"))
  (:`Pressed`
    (bind _returnvalue (`|CreateWidget` "/Game/character/blueprints/UI/pause.pause_C" (`GameplayStatics.GetPlayerController` 0)))
    (`UserWidget.AddToViewport` _returnvalue 0)))

(event `self.ReceiveTick`
  (params (DeltaSeconds :type "Float (single-precision)"))
  (if (== (`self.score`) (`self.win_score`))
    (bind _returnvalue (`|CreateWidget` "/Game/character/blueprints/UI/victory.victory_C"))
    (`UserWidget.AddToViewport` _returnvalue 0)
    (`GameplayStatics.SetGamePaused` true)
    (set `PlayerController.bShowMouseCursor` true (`GameplayStatics.GetPlayerController` 0))
    (set `self.lives` (+ (`self.lives`) 1))))

(event `self.ReceiveBeginPlay`
  (set `self.win_score` 1610))

(event `InputAxis|move down`
  (params (AxisValue :type "Float (single-precision)"))
  (`self.AddMovementInput` (* (`SceneComponent.GetRightVector` (`self.Sphere`)) (-1.0 -1.0 -1.0)) AxisValue))

(event `InputAxis|move right`
  (params (AxisValue :type "Float (single-precision)"))
  (`self.AddMovementInput` (* (`SceneComponent.GetForwardVector` (`self.Sphere`)) (-1.0 -1.0 -1.0)) AxisValue))

(event `InputAxis|move forward`
  (params (AxisValue :type "Float (single-precision)"))
  (`self.AddMovementInput` (`SceneComponent.GetRightVector` (`self.Sphere`)) AxisValue))

(event `InputAxis|move left`
  (params (AxisValue :type "Float (single-precision)"))
  (`self.AddMovementInput` (`SceneComponent.GetForwardVector` (`self.Sphere`)) AxisValue))

(fn `UserConstructionScript`)