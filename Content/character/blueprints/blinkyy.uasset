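; Blinkyy is an AI-moved enemy that wanders between waypoints and ends the game when it registers a hit.
; From BeginPlay it sends itself to a random Waypoint actor, repeating after a short delay on each successful move, with no handling for failed moves.
; Any Hit, with no check on the other actor, pauses the game, sets mouse cursor visibility and shows the Game_over widget.
; The patrol function is empty.
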(event `self.ReceiveHit`
  (params (MyComp :type "PrimitiveComponent Object Reference") (Other :type "Actor Object Reference") (OtherComp :type "PrimitiveComponent Object Reference") (bSelfMoved :type Boolean) (HitLocation :type "Vector Structure") (HitNormal :type "Vector Structure") (NormalImpulse :type "Vector Structure") (Hit :type "HitResult Structure (by ref)"))
  (bind _returnvalue (`GameplayStatics.SetGamePaused` true))
  (set `PlayerController.bShowMouseCursor` _returnvalue (`GameplayStatics.GetPlayerController` 0))
  (bind _returnvalue_2 (`|CreateWidget` "/Game/character/blueprints/UI/game_over.game_over_C"))
  (`UserWidget.AddToViewport` _returnvalue_2 0))

(event `self.ReceiveBeginPlay`
  (bind _outactors (`GameplayStatics.GetAllActorsOfClass` "/Game/character/blueprints/waypoint.waypoint_C" :!label _label))
  (`KismetSystemLibrary.Delay` 0.1)
  (`|AIMoveTo` self (0.0 0.0 0.0) (`KismetArrayLibrary.Array_Random` _outactors)
    (:`OnSuccess`
      (`KismetSystemLibrary.Delay` 0.1)
      (goto _label))))

(fn `patrol`)

(fn `UserConstructionScript`)